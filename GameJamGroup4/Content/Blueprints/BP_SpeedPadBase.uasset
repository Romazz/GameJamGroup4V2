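; Base Blueprint for speed pads that change the speed of the physics ball.
; Helper functions send speed-up and speed-down messages carrying a SpeedChange value, plus a stop message, to a given actor.
; Its begin and end overlap events filter for PhysicsBallBP and only print debug text; none of the helpers are called here.
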(event `self.ReceiveActorBeginOverlap`
  (params (OtherActor :type "Actor Object Reference"))
  (cast `/Game/RollingBP/Blueprints/PhysicsBallBP` OtherActor)
  (`KismetSystemLibrary.PrintString` "Entered"))

(event `self.ReceiveActorEndOverlap`
  (params (OtherActor :type "Actor Object Reference"))
  (cast `/Game/RollingBP/Blueprints/PhysicsBallBP` OtherActor)
  (`KismetSystemLibrary.PrintString` "Exited"))

(fn `SendSpeedDownMessage`
  (params (actorToSpeedDown :type "Actor Object Reference"))
  (message `/Game/Interfaces/iSpeedChangeable.SpeedDown` actorToSpeedDown (`self.speedChange`)))

(fn `SendSpeedUpMessage`
  (params (actorToSpeedUp :type "Actor Object Reference"))
  (message `/Game/Interfaces/iSpeedChangeable.SpeedUp` actorToSpeedUp (`self.speedChange`)))

(fn `SendStopSpeedChangeMessage`
  (params (actorToStopSpeedChange :type "Actor Object Reference"))
  (message `/Game/Interfaces/iSpeedChangeable.StopSpeedChange` actorToStopSpeedChange))

(fn `UserConstructionScript`)